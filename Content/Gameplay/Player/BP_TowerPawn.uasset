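; Player pawn, apparently for a tower game, that sets up the player HUD, handles the pause menu and holds the player's money.
; On BeginPlay it creates the HUD widget and adds it to the viewport.
; The Escape action drives a FlipFlop that alternately opens a new pause menu and removes it, switching game pause, input mode and mouse cursor to match.
; AddMoney adds the given amount to the Money total.
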(event EventBeginPlay
  (bind _returnvalue (UserInterface|CreateWidget "/Game/Gameplay/WBP_PlayerHUD.WBP_PlayerHUD_C"))
  (UserInterface|Viewport|AddtoViewport _returnvalue 0))

(event Collision|EventActorBeginOverlap
  (params (OtherActor :type Actor%20Object%20Reference)))

(event EventTick
  (params (DeltaSeconds :type Float%20%28single-precision%29)))

(event Input|ActionEvents|InputActionEscapePressed
  (params (Key :type Key%20Structure :default "None"))
  (bind _returnvalue (Game|GetPlayerController 0))
  (bind _returnvalue_2 (Game|GetPlayerController 0))
  (:Pressed
    (Utilities|FlowControl|FlipFlop
      (:A
        (bind _returnvalue_3 (UserInterface|CreateWidget "/Game/UI/PauseMenu.PauseMenu_C"))
        (UserInterface|Viewport|AddtoViewport _returnvalue_3 0)
        (Game|SetGamePaused true)
        (Input|SetInputModeGameandUI _returnvalue 0 "DoNotLock" true false)
        (Variables|/Script/Engine.PlayerController|SetbShowMouseCursor _returnvalue true))
      (:B
        (Widget|RemovefromParent _returnvalue_3)
        (Input|SetInputModeGameOnly _returnvalue_2 false)
        (Variables|/Script/Engine.PlayerController|SetbShowMouseCursor _returnvalue_2 false)
        (Game|SetGamePaused false)))))

(fn ConstructionScript)

(fn AddMoney
  (params (moneyToAdd :type Integer))
  (Variables|Default|Setmoney (+ moneyToAdd (Variables|Default|Getmoney))))