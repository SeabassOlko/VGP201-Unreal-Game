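; Actor component that tracks round progress and live enemy count for its owning BP_EnemySpawner.
; RunRound passes the current round number and enemies-per-round count to the spawner, which it caches on BeginPlay.
; Increment and decrement functions maintain the spawned-enemy count and advance the round, clamped to a maximum.
; Tick polls for spawning finished with no enemies left, then tells the spawner to reset the running round.
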(event Custom|RunRound
  (Default|Set/StartRound (Variables|Default|GetEnemySpawner) (Variables|Default|GetCurrentRound) (Variables|Default|GetEnemiesPerRound)))

(event EventTick
  (params (DeltaSeconds :type Float%20%28single-precision%29))
  (if (Variables|Default|GetSpawningFinished)
    (if (not (> (Variables|Default|GetEnemiesSpawned) 0))
      (Default|ResetRunningRound (Variables|Default|GetEnemySpawner)))))

(event EventBeginPlay
  (bind _asbp_enemy_spawner (Utilities|Casting|CastToBP_EnemySpawner (Components|GetOwner)))
  (Variables|Default|SetEnemySpawner _asbp_enemy_spawner))

(fn IncrementEnemiesSpawned
  (bind _result (Math|Integer|IncrementInt (Variables|Default|GetEnemiesSpawned))
    (:%20%20
      (Variables|Default|SetEnemiesSpawned _result))))

(fn DecrementEnemiesSpawned
  (bind _result (Math|Integer|DecrementInt (Variables|Default|GetEnemiesSpawned))
    (:%20%20
      (Variables|Default|SetEnemiesSpawned _result))))

(fn IncrementRound
  (bind _result (Math|Integer|IncrementInt (Variables|Default|GetCurrentRound))
    (:%20%20
      (Variables|Default|SetCurrentRound (Math|Integer|Clamp(Integer) _result 0 (Variables|Default|GetMaxRounds))))))