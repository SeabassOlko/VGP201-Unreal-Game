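; BP_SplinePath is a spline-based path actor that draws itself with meshes and exposes its spline to other code.
; The construction script adds one spline mesh component per segment, aligned on the X axis and bent using the local positions and tangents of each pair of neighboring points.
; GetSpline returns the SplinePath component.
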(fn ConstructionScript
  (bind _splinepath (Variables|Default|GetSplinePath))
  (for _index (range 0 (- (Spline|GetNumberOfSplinePoints (Variables|Default|GetSplinePath)) 2))
    (bind _returnvalue (AddComponent|AddSplineMeshComponent false))
    (SplineMesh|SetForwardAxis _returnvalue "X" true)
    (SplineMesh|SetStartandEnd _returnvalue (Spline|GetLocationatSplinePoint _splinepath _index "Local") (Spline|GetTangentatSplinePoint _splinepath _index "Local") (Spline|GetLocationatSplinePoint _splinepath (+ _index 1) "Local") (Spline|GetTangentatSplinePoint _splinepath (+ _index 1) "Local") true :!class /Script/Engine.SplineMeshComponent)))

(fn GetSpline
  (return (Variables|Default|GetSplinePath)))