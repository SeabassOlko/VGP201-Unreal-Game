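; BP_Enemy is a slow-walking enemy pawn that heads for a goal and damages the player's tower.
; On BeginPlay, after a short delay, it lowers its walk speed and uses AI MoveTo toward a randomly indexed BP_Goal actor.
; Both move success and failure subtract its Damage from the BP_TowerPawn player's Health, then destroy the enemy after a delay.
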(event EventBeginPlay
  (Utilities|FlowControl|Delay 0.2)
  (Variables|/Script/Engine.CharacterMovementComponent|SetMaxWalkSpeed (Variables|Character|GetCharacterMovement) 25.0)
  (bind _outactors (Actor|GetAllActorsOfClass "/Game/Gameplay/BP_Goal.BP_Goal_C"))
  (AI|AIMoveTo self "0, 0, 0" (Utilities|Array|Get(acopy) _outactors (Math|Random|RandomIntegerinRange 0 (Utilities|Array|Length _outactors))) 5.0 false
    (:OnSuccess
      _)
    (:OnFail
      _))
  (bind _astower_pawn (Utilities|Casting|CastToBP_TowerPawn (Game|Player|GetPlayerPawn 0)))
  (Variables|/Game/Gameplay/Player/BP_TowerPawn.BP_TowerPawn_C|SetHealth _astower_pawn (- (Variables|/Game/Gameplay/Player/BP_TowerPawn.BP_TowerPawn_C|GetHealth _astower_pawn) (Variables|Default|GetDamage)))
  (Utilities|FlowControl|Delay 3.0)
  (Actor|DestroyActor))

(event Collision|EventActorBeginOverlap
  (params (OtherActor :type Actor%20Object%20Reference)))

(event EventTick
  (params (DeltaSeconds :type Float%20%28single-precision%29)))

(fn ConstructionScript
  (|CallParentFunction))