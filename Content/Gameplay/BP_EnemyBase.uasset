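; BP_EnemyBase is an enemy base Blueprint that handles death and the money reward to the player.
; Tick polls Health every frame and, at zero or below, calls DestroyActor before casting player pawn 0 to BP_TowerPawn.
; A successful cast adds EnemyValue through AddMoney and sets IsDead, while a failed one only prints an error.
; While Health stays positive, IsDead is reset to false each frame.
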(event EventBeginPlay)

(event Collision|EventActorBeginOverlap
  (params (OtherActor :type Actor%20Object%20Reference)))

(event EventTick
  (params (DeltaSeconds :type Float%20%28single-precision%29))
  (if (<= (Variables|Default|GetHealth) 0.0)
    (Actor|DestroyActor)
    (bind _asbp_tower_pawn (Utilities|Casting|CastToBP_TowerPawn (Game|Player|GetPlayerPawn 0))
      (:then
        (Default|AddMoney _asbp_tower_pawn (Variables|Default|GetenemyValue))
        (Variables|Default|SetisDead true))
      (:CastFailed
        (Development|PrintString "Cast to BP_TowerPawn failed" true true "(R=1.000000,G=0.100903,B=0.000000,A=1.000000)")))
    (else
      (Variables|Default|SetisDead false))))

(fn ConstructionScript)