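; Enemy spawner that spawns each round's enemies and sends them along spline paths.
; SetStartRound starts a self-calling RunRound loop, with delays between spawns that shrink as rounds rise.
; Round number and a cycling counter pick Blue, Yellow or Red enemies, shifting to all Red after round nine.
; Spawns rotate through SplinePaths and report to ACRoundManager, which increments the round when the loop ends.
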(event Custom|RunRound
  (bind _self self)
  (bind _splinepaths (Variables|Default|GetSplinePaths))
  (bind _roundnumber (Variables|Default|GetRoundNumber))
  (bind _returnvalue (Transformation|GetActorTransform _self))
  (Variables|Default|SetRunningRound true)
  (if (Variables|Default|GetFirstSpawn)
    (Variables|Default|SetFirstSpawn false)
    (else
      (Utilities|FlowControl|Delay (/ 5.0 (Math|Conversions|ToFloat(Integer) (Variables|Default|GetRoundNumber))))))
  (bind _result (Math|Integer|IncrementInt (Variables|Default|GetEnemiesSpawned))
    (:%20%20
      (Variables|Default|SetEnemiesSpawned _result)
      (if (<= _roundnumber 3)
        (bind _returnvalue_2 (Game|SpawnActorfromClass "/Game/Characters/Enemies/BP_EnemyBlue.BP_EnemyBlue_C" _returnvalue "Undefined" "MultiplyWithRoot" 0 0 :!label _label))
        (Variables|Default|SetCurrentEnemy _returnvalue_2)
        (elif (<= _roundnumber 6)
          (if (<= (Variables|Default|GetEnemyTypeCount) 3)
            (goto _label)
            (else
              (bind _returnvalue_3 (Game|SpawnActorfromClass "/Game/Characters/Enemies/BP_EnemyYellow.BP_EnemyYellow_C" _returnvalue "Undefined" "MultiplyWithRoot" 0 0 :!label _label_2))
              (Variables|Default|SetCurrentEnemy _returnvalue_3)))
          (else
            (if (<= _roundnumber 9)
              (if (<= (Variables|Default|GetEnemyTypeCount) 3)
                (goto _label)
                (elif (<= (Variables|Default|GetEnemyTypeCount) 6)
                  (goto _label_2)
                  (else
                    _))))
            (bind _returnvalue_4 (Game|SpawnActorfromClass "/Game/Characters/Enemies/BP_EnemyRed.BP_EnemyRed_C" _returnvalue "Undefined" "MultiplyWithRoot" 0 0))
            (Variables|Default|SetCurrentEnemy _returnvalue_4))))
      (bind _result_2 (Math|Integer|IncrementInt (Variables|Default|GetEnemyTypeCount))
        (:%20%20
          (Variables|Default|SetEnemyTypeCount _result_2)
          (Default|IncrementEnemiesSpawned (Variables|Default|GetAC_RoundManager))
          (Default|SetSpline (Variables|/Game/Characters/Enemies/BP_EnemyBase.BP_EnemyBase_C|GetAC_EnemyMovement (Variables|Default|GetCurrentEnemy)) (Variables|/Game/Gameplay/BP_SplinePath.BP_SplinePath_C|GetSplinePath (Utilities|Array|Get(acopy) _splinepaths (Math|Integer|%(Integer) (Variables|Default|GetEnemiesSpawned) (Utilities|Array|Length _splinepaths)))))
          (if (>= (Variables|Default|GetEnemyTypeCount) (Variables|Default|GetRoundNumber))
            (Variables|Default|SetEnemyTypeCount 0))
          (if (<= (Variables|Default|GetEnemiesSpawned) (Variables|Default|GetEnemiesToSpawn))
            (CallFunction|RunRound)
            (else
              (Variables|Default|SetEnemiesSpawned 1)
              (Variables|Default|SetFirstSpawn true)
              (Default|IncrementRound (Variables|Default|GetAC_RoundManager)))))))))

(event Custom|CallRoundManager
  (Default|RunRound (Variables|Default|GetAC_RoundManager)))

(fn ConstructionScript)

(fn Set/StartRound
  (params (RoundNumber :type Integer) (EnemiesToSpawn :type Integer))
  (Variables|Default|SetRoundNumber RoundNumber)
  (Variables|Default|SetEnemiesToSpawn EnemiesToSpawn)
  (CallFunction|RunRound))

(fn ResetRunningRound
  (Variables|Default|SetRunningRound false))