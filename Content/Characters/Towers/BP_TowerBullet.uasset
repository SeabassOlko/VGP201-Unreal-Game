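; BP_TowerBullet is a placeable tower that automatically shoots enemies within its range collider, damaging them directly without spawning projectiles.
; Once placed, overlap events maintain a target list; Tick turns the turret toward the first target and calls Shoot.
; Shoot uses Delays to pace damage and muzzle flash, scaling fire rate and clamped damage by tower tier.
; Before placement, Tick swaps mesh materials to red outside placeable areas.
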(event OnComponentBeginOverlap(TurretRangeCollider)
  (params (OverlappedComponent :type Primitive%20Component%20Object%20Reference) (OtherActor :type Actor%20Object%20Reference) (OtherComp :type Primitive%20Component%20Object%20Reference) (OtherBodyIndex :type Integer) (bFromSweep :type Boolean) (SweepResult :type Hit%20Result%20Structure%20%28by%20ref%29))
  ;[1 1 1] When enemy enters collider, add enemy to list of targets
  (if (Variables|Default|GetPlaced)
    (bind _asbp_enemy_base (Utilities|Casting|CastToBP_EnemyBase OtherActor))
    (Utilities|Array|Add (Variables|Default|GetTargets) _asbp_enemy_base)))

(event OnComponentEndOverlap(TurretRangeCollider)
  (params (OverlappedComponent :type Primitive%20Component%20Object%20Reference) (OtherActor :type Actor%20Object%20Reference) (OtherComp :type Primitive%20Component%20Object%20Reference) (OtherBodyIndex :type Integer))
  ;[1 1 1] When enemy leaves collider, remove from target list
  (if (Variables|Default|GetPlaced)
    (bind _asbp_enemy_base (Utilities|Casting|CastToBP_EnemyBase OtherActor))
    (Utilities|Array|RemoveItem (Variables|Default|GetTargets) _asbp_enemy_base)))

(event EventBeginPlay
  ;[1 1 1] Create an array of the meshes for easier material changing
  (|CallParentFunction)
  (Variables|Default|SetArrayOfTowerMeshes (Utilities|Array|MakeArray (Variables|Default|GetTurret) (Variables|Default|GetCylinder) (Variables|Default|GetBody))))

(event EventTick
  (params (DeltaSeconds :type Float%20%28single-precision%29))
  (|CallParentFunction DeltaSeconds)
  (if (Variables|Default|GetPlaced)
    ;[1 1 1] If turret has targets, face the first target in list and shoot at it
    (if (> (Utilities|Array|Length (Variables|Default|GetTargets)) 0)
      (CallFunction|LookatEnemy)
      (Utilities|Shoot))
    (else
      ;[1 1 1] If not placed check and change material based on collisions
      (CallFunction|ChangeMaterialonCollision))))

(fn ConstructionScript
  (|CallParentFunction))

(fn ChangeMaterialonCollision
  (bind _arrayoftowermeshes (Variables|Default|GetArrayOfTowerMeshes))
  (if (Variables|Default|GetPlaceableArea)
    ;[1 1 1] If in placable area have normal material set
    (for _array_element _arrayoftowermeshes
      (Rendering|Material|SetMaterial _array_element 0 "/Game/Materials/TowerMaterials/M_TowerBaseMaterial.M_TowerBaseMaterial"))
    (else
      ;[1 1 1] If not placable switch to red material
      (for _array_element_2 _arrayoftowermeshes
        (Rendering|Material|SetMaterial _array_element_2 0 "/Game/Materials/TowerMaterials/MI_TowerUnPlacableMaterial.MI_TowerUnPlacableMaterial")))))

(fn LookatEnemy
  (bind _returnvalue (Transformation|GetActorLocation))
  (bind _targets (Variables|Default|GetTargets))
  (bind _output (Utilities|Array|Get(acopy) _targets))
  (bind _returnvalue_2 (Transformation|GetActorLocation _output))
  ;[1 1 1] Rotate turret to face enemy
  (Transformation|SetRelativeRotation (Variables|Default|GetTurret) (Math|Rotator|FindLookatRotation (Math|Vector|MakeVector (.x _returnvalue) (.y _returnvalue) 0.0) (Math|Vector|MakeVector (.x _returnvalue_2) (.y _returnvalue_2) 0.0)) false false))