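; Base tower actor for placeable towers, handling cursor-driven placement and tiered upgrades.
; Until placed, it follows the cursor trace at a fixed height, while an overlap counter on its placement box sets PlaceableArea, filtering out itself, floor-tagged actors and, on begin overlap, turret range colliders.
; Its upgrade widget component receives the tower as owner and starts hidden.
; Upgrading raises the tier and swaps mesh materials, hiding the widget from tier three.
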(event OnComponentBeginOverlap(PlacementCollisionBox)
  (params (OverlappedComponent :type Primitive%20Component%20Object%20Reference) (OtherActor :type Actor%20Object%20Reference) (OtherComp :type Primitive%20Component%20Object%20Reference) (OtherBodyIndex :type Integer) (bFromSweep :type Boolean) (SweepResult :type Hit%20Result%20Structure%20%28by%20ref%29))
  (if (Utilities|Enum|NotEqual(Enum) (Utilities|GetObjectName OtherComp) "TurretRangeCollider")
    (bind _returnvalue (CallFunction|CheckPlacementCollisions OtherActor))
    (if _returnvalue
      (bind _result (Math|Integer|IncrementInt (Variables|Default|GetCollisions))
        (:%20%20
          (Variables|Default|SetCollisions _result)
          (Variables|Default|SetPlaceableArea false))))))

(event OnComponentEndOverlap(PlacementCollisionBox)
  (params (OverlappedComponent :type Primitive%20Component%20Object%20Reference) (OtherActor :type Actor%20Object%20Reference) (OtherComp :type Primitive%20Component%20Object%20Reference) (OtherBodyIndex :type Integer))
  (bind _returnvalue (CallFunction|CheckPlacementCollisions OtherActor))
  (if _returnvalue
    (bind _result (Math|Integer|DecrementInt (Variables|Default|GetCollisions))
      (:%20%20
        (bind _output_get (Variables|Default|SetCollisions _result))
        (if (<= _output_get 0)
          (Variables|Default|SetPlaceableArea true))))))

(event EventBeginPlay
  (bind _aswbp_upgrade_widget (Utilities|Casting|CastToWBP_UpgradeWidget (UserInterface|GetWidget (Variables|Default|GetUpgradeWidgetComponent))))
  (Default|SetTowerOwner _aswbp_upgrade_widget self)
  (CallFunction|TurnOffUpgradeWidget))

(event EventTick
  (params (DeltaSeconds :type Float%20%28single-precision%29))
  (bind _returnvalue (Game|GetPlayerController 0))
  (bind _array (Utilities|Array|MakeArray "ObjectTypeQuery1"))
  (bind _hitresult (Class|PlayerController|GetHitResultUnderCursorforObjects _returnvalue _array true))
  (bind _location (Collision|BreakHitResult _hitresult))
  (if (not (Variables|Default|GetPlaced))
    (Transformation|SetActorLocation self (Math|Vector|MakeVector (.x _location) (.y _location) 74.0) false false)))

(fn ConstructionScript)

(fn CheckPlacementCollisions
  (params (Collision :type Actor%20Object%20Reference))
  (return (and (!= self Collision) (!= (Utilities|Array|Get(acopy) (Variables|/Script/Engine.Actor|GetTags Collision)) "Floor"))))

(fn TurnOffUpgradeWidget
  (Development|SetHiddeninGame (Variables|Default|GetUpgradeWidgetComponent) true false))

(fn TurnonUpgradeWidget
  (Development|SetHiddeninGame (Variables|Default|GetUpgradeWidgetComponent) false false))

(fn UpgradeTower
  (bind _arrayoftowermeshes (Variables|Default|GetArrayOfTowerMeshes))
  (bind _result (Math|Integer|IncrementInt (Variables|Default|GetTowerTier))
    (:%20%20
      (bind _output_get (Variables|Default|SetTowerTier _result))
      (if (< _output_get 3)
        (for _array_element _arrayoftowermeshes
          (Rendering|Material|SetMaterial _array_element 0 "/Game/Materials/TowerMaterials/MI_TowerUpgrade1Material.MI_TowerUpgrade1Material"))
        (else
          (for _array_element_2 _arrayoftowermeshes
            (Rendering|Material|SetMaterial _array_element_2 0 "/Game/Materials/TowerMaterials/MI_TowerUpgrade2Material.MI_TowerUpgrade2Material"))
          (CallFunction|TurnOffUpgradeWidget))))))