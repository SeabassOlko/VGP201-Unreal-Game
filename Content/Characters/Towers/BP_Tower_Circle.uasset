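; Tower-defense turret that, once placed, damages enemies in eight barrel range colliders while the spawner's round is running.
; Before placement, Tick swaps its mesh materials to show whether the spot is placeable.
; Tick calls Shoot, whose Delay paces firing by fire rate over tier, then applies clamped, tier-scaled damage to overlapping enemies and blinks the muzzle flashes.
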(event EventBeginPlay
  (|CallParentFunction)
  (CallFunction|Innit))

(event EventTick
  (params (DeltaSeconds :type Float%20%28single-precision%29))
  (|CallParentFunction DeltaSeconds)
  ;[1 1 1] If placed, check if round is running and fire constantly
  (if (Variables|Default|GetPlaced)
    (if (Variables|/Game/Gameplay/BP_EnemySpawner.BP_EnemySpawner_C|GetRunningRound (Variables|Default|GetSpawnerRef))
      (Utilities|Shoot))
    (else
      ;[1 1 1] Otherwise change materials when colliding
      (CallFunction|ChangeMaterialonCollision))))

(fn ConstructionScript
  (|CallParentFunction))

(fn ChangeMaterialonCollision
  (bind _arrayoftowermeshes (Variables|Default|GetArrayOfTowerMeshes))
  (if (Variables|Default|GetPlaceableArea)
    ;[1 1 1] If in placable area change to normal material
    (for _array_element _arrayoftowermeshes
      (Rendering|Material|SetMaterial _array_element 0 "/Game/Materials/TowerMaterials/M_TowerBaseMaterial.M_TowerBaseMaterial"))
    (else
      ;[1 1 1] If not placable area then change to red material
      (for _array_element_2 _arrayoftowermeshes
        (Rendering|Material|SetMaterial _array_element_2 0 "/Game/Materials/TowerMaterials/MI_TowerUnPlacableMaterial.MI_TowerUnPlacableMaterial")))))

(fn Innit
  (Variables|Default|SetArrayOfTowerMeshes (Utilities|Array|MakeArray (Variables|Default|GetBody) (Variables|Default|GetTop) (Variables|Default|GetBarrel) (Variables|Default|GetBarrel1) (Variables|Default|GetBarrel2) (Variables|Default|GetBarrel3)))
  (Variables|Default|SetRangeBoxCollisionArray (Utilities|Array|MakeArray (Variables|Default|GetBarrelRangeCollider) (Variables|Default|GetBarrelRangeCollider1) (Variables|Default|GetBarrelRangeCollider2) (Variables|Default|GetBarrelRangeCollider3) (Variables|Default|GetBarrelRangeCollider4) (Variables|Default|GetBarrelRangeCollider5) (Variables|Default|GetBarrelRangeCollider6) (Variables|Default|GetBarrelRangeCollider7)))
  (Variables|Default|SetMuzzleFlashArray (Utilities|Array|MakeArray (Variables|Default|GetMuzzleFlash) (Variables|Default|GetMuzzleFlash1) (Variables|Default|GetMuzzleFlash2) (Variables|Default|GetMuzzleFlash3) (Variables|Default|GetMuzzleFlash4) (Variables|Default|GetMuzzleFlash5) (Variables|Default|GetMuzzleFlash6) (Variables|Default|GetMuzzleFlash7)))
  ;[1 1 1] Get spawner ref to know when round is running
  (bind _outactors (Actor|GetAllActorsOfClass "/Game/Gameplay/BP_EnemySpawner.BP_EnemySpawner_C"))
  (Variables|Default|SetSpawnerRef (Utilities|Array|Get(acopy) _outactors)))