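; Actor component that moves a BP_EnemyBase owner along a spline path.
; SetSpline stores the spline and runs Init, which caches the owner, sets its timeline's play rate from TimelineLength, and starts it.
; RunSplineMovement lerps spline distance by the owner's Alpha, setting location and rotation from the spline while keeping the enemy's current Z height.
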(event Custom|RunSplineMovement
  (bind _splinepathref (Variables|Default|GetSplinePathRef))
  (bind _splinepathref_2 (Variables|Default|GetSplinePathRef))
  (bind _enemybaseref (Variables|Default|GetEnemyBaseRef))
  (bind _enemybaseref_2 (Variables|Default|GetEnemyBaseRef))
  (bind _returnvalue (Spline|GetSplineLength _splinepathref))
  (bind _alpha (Variables|/Game/Characters/Enemies/BP_EnemyBase.BP_EnemyBase_C|GetAlpha _enemybaseref_2))
  (bind _returnvalue_2 (Math|Float|Lerp 0.0 _returnvalue _alpha))
  (bind _returnvalue_3 (Spline|GetLocationatDistanceAlongSpline _splinepathref_2 _returnvalue_2 "World"))
  ;[1 1 1] Set the enemies location and rotation, keeping its original Z height
  (Transformation|SetActorLocationAndRotation _enemybaseref (Math|Vector|MakeVector (.x _returnvalue_3) (.y _returnvalue_3) (.z (Transformation|GetActorLocation _enemybaseref))) (Spline|GetRotationatDistanceAlongSpline _splinepathref_2 _returnvalue_2 "World")))

(fn SetSpline
  (params (SplineRef :type Spline%20Component%20Object%20Reference))
  ;[1 1 1] Sets the spline path ref then initializes the rest of the component
  (Variables|Default|SetSplinePathRef SplineRef)
  (CallFunction|Init))

(fn Init
  ;[1 1 1] Get a reference of the timeline from the owning enemy
  (bind _asbp_enemy_base (Utilities|Casting|CastToBP_EnemyBase (Components|GetOwner))
    (:then
      (bind _output_get (Variables|Default|SetEnemyBaseRef _asbp_enemy_base))
      (bind _timeline (Default|GetTimeline _output_get))
      (bind _output_get_2 (Variables|Default|SetTimelineRef _timeline))
      (Components|Timeline|SetPlayRate _output_get_2 (/ 1.0 (Variables|Default|GetTimelineLength)))
      ;[1 1 1] Starts running the timeline in the owning enemy
      (Default|StartTimeline (Variables|Default|GetEnemyBaseRef))
      (return))
    (:CastFailed
      (Development|PrintString "Could not cast to BP_EnemyBase" true true "(R=1.000000,G=0.000000,B=0.075233,A=1.000000)"))))