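; Base enemy for a tower defense game that travels along a spline, takes damage and pays out money when killed.
; A timeline supplies the alpha that its movement component uses for spline movement; finishing it damages the tower pawn and removes the enemy.
; Any damage lowers clamped health, which Tick polls to destroy the enemy and award money.
; Both exits decrement the spawner's round manager count.
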(event Custom|StartTimeline
  (bind _alpha (Timeline|MovementTimeline PlayFromStart)
    (:Update
      ;[1 1 1] Set the alpha to be used in spline movement
      (Variables|Default|SetAlpha _alpha)
      (Default|RunSplineMovement (Variables|Default|GetAC_EnemyMovement)))
    (:Finished
      ;[1 1 1] Once end of timeline reached, damage the player and destroy/decrement the enemy
      (bind _asbp_tower_pawn (Utilities|Casting|CastToBP_TowerPawn (Game|Player|GetPlayerPawn 0)))
      (Default|DamagePlayer _asbp_tower_pawn (Variables|Default|GetDamage))
      (bind _returnvalue (Actor|GetActorOfClass "/Game/Gameplay/BP_EnemySpawner.BP_EnemySpawner_C"))
      (Default|DecrementEnemiesSpawned (Variables|/Game/Gameplay/BP_EnemySpawner.BP_EnemySpawner_C|GetAC_RoundManager _returnvalue))
      (Actor|DestroyActor))))

(event Game|Damage|EventAnyDamage
  (params (Damage :type Float%20%28single-precision%29) (DamageType :type Damage%20Type%20Object%20Reference) (InstigatedBy :type Controller%20Object%20Reference) (DamageCauser :type Actor%20Object%20Reference))
  (CallFunction|TakeDamage Damage))

(event EventTick
  (params (DeltaSeconds :type Float%20%28single-precision%29))
  (if (<= (Variables|Default|GetHealth) 0.0)
    ;[1 1 1] Destroy Enemy and add money to player
    (Actor|DestroyActor)
    (bind _asbp_tower_pawn (Utilities|Casting|CastToBP_TowerPawn (Game|Player|GetPlayerPawn 0))
      (:then
        (Default|AddMoney _asbp_tower_pawn (Variables|Default|GetenemyValue))
        ;[1 1 1] Decrement Enemy from round manager
        (bind _returnvalue (Actor|GetActorOfClass "/Game/Gameplay/BP_EnemySpawner.BP_EnemySpawner_C"))
        (Default|DecrementEnemiesSpawned (Variables|/Game/Gameplay/BP_EnemySpawner.BP_EnemySpawner_C|GetAC_RoundManager _returnvalue))
        (Variables|Default|SetisDead true))
      (:CastFailed
        (Development|PrintString "Cast to BP_TowerPawn failed" true true "(R=1.000000,G=0.100903,B=0.000000,A=1.000000)")))
    (else
      (Variables|Default|SetisDead false))))

(fn ConstructionScript)

(fn GetTimeline
  ;[1 1 1] Used to bring timeline into movement component
  (return (Variables|Default|GetMovementTimeline)))

(fn TakeDamage
  (params (DamageAmt :type Float%20%28double-precision%29))
  ;[1 1 1] Subtract from enemy health, and clamp to not go lower than 0
  (Variables|Default|SetHealth (Math|Float|Clamp(Float) (- (Variables|Default|GetHealth) DamageAmt) 0.0 1.5e+02)))