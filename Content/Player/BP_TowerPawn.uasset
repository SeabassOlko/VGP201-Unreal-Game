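; Player pawn for a tower defense game, tracking money and health and creating the HUD with a reference to the enemy spawner.
; Left click places a held tower on valid ground or cursor-traces for a tower to show its upgrade widget, while right click refunds a held tower.
; Escape toggles the pause menu via FlipFlop, Tick calls LoseGame at zero health, and WinGame and LoseGame pause and swap in end screens.
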(event EventBeginPlay
  ;[1 1 1] Set starting values of the player
  (Variables|Default|SetMoney (Variables|Default|GetStartingMoney))
  (Variables|Default|SetHealth (Variables|Default|GetMaxHealth))
  ;[1 1 1] Create HUD widget and pass reference to the enemy spawner for the start button
  (bind _returnvalue (UserInterface|CreateWidget "/Game/UI/InGame_UI/WBP_PlayerHUD.WBP_PlayerHUD_C"))
  (bind _returnvalue_2 (Actor|GetActorOfClass "/Game/Gameplay/BP_EnemySpawner.BP_EnemySpawner_C"))
  (Variables|/Game/UI/InGame_UI/WBP_PlayerHUD.WBP_PlayerHUD_C|SetEnemySpawner _returnvalue _returnvalue_2)
  (UserInterface|Viewport|AddtoViewport _returnvalue 0)
  (Variables|/Script/Engine.PlayerController|SetbShowMouseCursor (Game|GetPlayerController 0) true))

(event EventTick
  (params (DeltaSeconds :type Float%20%28single-precision%29))
  ;[1 1 1] Checks if the player has run out of health, if yes then the game is over
  (if (<= (Variables|Default|GetHealth) 0)
    (CallFunction|LoseGame)))

(event Input|ActionEvents|InputActionEscapePressed
  (params (Key :type Key%20Structure :default "None"))
  (bind _returnvalue (Game|GetPlayerController 0))
  (bind _returnvalue_2 (Game|GetPlayerController 0))
  (:Pressed
    (Utilities|FlowControl|FlipFlop
      (:A
        ;[1 1 1] First press of pause button will create the pause widget and add to the player and pause the game
        (bind _returnvalue_3 (UserInterface|CreateWidget "/Game/UI/Menu_UI/WBP_PauseMenu.WBP_PauseMenu_C"))
        (UserInterface|Viewport|AddtoViewport _returnvalue_3 0)
        (Game|SetGamePaused true)
        (Input|SetInputModeGameandUI _returnvalue 0 "DoNotLock" true false)
        (Variables|/Script/Engine.PlayerController|SetbShowMouseCursor _returnvalue true))
      (:B
        ;[1 1 1] Second press will remove the pause menu widget from the player and unpause the game
        (Widget|RemovefromParent _returnvalue_3)
        (Input|SetInputModeGameOnly _returnvalue_2 false)
        (Variables|/Script/Engine.PlayerController|SetbShowMouseCursor _returnvalue_2 true)
        (Game|SetGamePaused false)))))

(event Input|ActionEvents|InputActionLeftMouseButtonPressed
  (params (Key :type Key%20Structure :default "None"))
  (:Pressed
    (if (Variables|Default|GetHoldingTower)
      ;[1 1 1] If holding tower and the tower is in a placable area, then place the tower and reset holding tower
      (if (Variables|/Game/Characters/Towers/BP_TowerBase.BP_TowerBase_C|GetPlaceableArea (Variables|Default|GetHeldTower))
        (Variables|/Game/Characters/Towers/BP_TowerBase.BP_TowerBase_C|SetPlaced (Variables|Default|GetHeldTower) true)
        (Variables|Default|SetHoldingTower false))
      (else
        ;[1 1 1] If the player is not holding a tower, check if they clicked on a tower to create upgrade UI
        (CallFunction|CheckTowerUnderClick)))))

(event Input|ActionEvents|InputActionRightMousButtonPressed
  (params (Key :type Key%20Structure :default "None"))
  ;[1 1 1] If the right mouse button is pressed while holding a tower, it is removed from the players control and the cost refunded
  (:Pressed
    (if (Variables|Default|GetHoldingTower)
      (Variables|Default|SetMoney (+ (Variables|Default|GetMoney) (Variables|/Game/Characters/Towers/BP_TowerBase.BP_TowerBase_C|GetTowerCost (Variables|Default|GetHeldTower))))
      (Actor|DestroyActor (Variables|Default|GetHeldTower))
      (Variables|Default|SetHoldingTower false))))

(fn ConstructionScript)

(fn AddMoney
  (params (moneyToAdd :type Integer))
  ;[1 1 1] Adds amount given to player money
  (Variables|Default|SetMoney (+ moneyToAdd (Variables|Default|GetMoney))))

(fn DamagePlayer
  (params (DamageAmount :type Integer))
  ;[1 1 1] Subtracts from player health damage amount before clamping to a minimun of 0
  (Variables|Default|SetHealth (Math|Integer|Clamp(Integer) (- (Variables|Default|GetHealth) DamageAmount) 0 (Variables|Default|GetMaxHealth))))

(fn SubtractMoney
  (params (Cost :type Integer))
  ;[1 1 1] Subtracts amount given from player money
  (Variables|Default|SetMoney (- (Variables|Default|GetMoney) Cost)))

(fn CheckTowerUnderClick
  ;[1 1 1] Get the actor under the mouse cursor and check if it is a tower
  (bind _asbp_tower_base (Utilities|Casting|CastToBP_TowerBase (.hitactor (.HitResult (Class|PlayerController|GetHitResultUnderCursorforObjects (Game|GetPlayerController 0) (Utilities|Array|MakeArray "ObjectTypeQuery3") true))))
    (:then
      ;[1 1 1] Check if tower clicked is not fully upgraded
      (if (< (Variables|/Game/Characters/Towers/BP_TowerBase.BP_TowerBase_C|GetTowerTier _asbp_tower_base) 3)
        ;[1 1 1] If another tower is selected, deselect previous tower
        (Utilities|IsValid (Variables|Default|GetSelectedTowerRef)
          (:Is%20Valid
            (Default|TurnOffUpgradeWidget (Variables|Default|GetSelectedTowerRef)))
          (:Is%20Not%20Valid
            _))
        ;[1 1 1] After set clicked tower as selected tower and turn on its upgrade widget
        (bind _output_get (Variables|Default|SetSelectedTowerRef _asbp_tower_base))
        (Default|TurnonUpgradeWidget _output_get)
        (Variables|Default|SetTowerSelected true)))
    (:CastFailed
      ;[1 1 1] When player did not click a tower, check if has tower selected  and unselect tower
      (Variables|Default|SetTowerSelected false)
      (Utilities|IsValid (Variables|Default|GetSelectedTowerRef)
        (:Is%20Valid
          (Default|TurnOffUpgradeWidget (Variables|Default|GetSelectedTowerRef)))))))

(fn WinGame
  ;[1 1 1] Pause the game, remove all previous widgets then create the win widget
  (Game|SetGamePaused true)
  (Viewport|RemoveAllWidgets)
  (bind _returnvalue (UserInterface|CreateWidget "/Game/UI/InGame_UI/WBP_YouWin.WBP_YouWin_C"))
  (UserInterface|Viewport|AddtoViewport _returnvalue 0))

(fn LoseGame
  ;[1 1 1] Pause the Game, remove all previous widgets then create the Game over Widget
  (Game|SetGamePaused true)
  (Viewport|RemoveAllWidgets)
  (bind _returnvalue (UserInterface|CreateWidget "/Game/UI/InGame_UI/WBP_GameOver.WBP_GameOver_C"))
  (UserInterface|Viewport|AddtoViewport _returnvalue 0))